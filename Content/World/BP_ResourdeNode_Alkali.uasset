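; BP_ResourdeNode_Alkali is a resource node that supplies an infinite amount of lithium ore at the node's own purity.
; On BeginPlay, only the authority initializes the resource and scatters the decorative PillsMesh instances.
; CreateInstances places them at random angles around the vertical axis, with the PileShape curve remapping random radial distance and random per-axis scaling varying each piece.
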(event EventBeginPlay
  (|CallParentFunction)
  (Networking|SwitchHasAuthority
    (:Authority
      (Class|FGResourceNode|InitResource "/Lithium/Resources/Lithium/Desc_OreLithium.Desc_OreLithium_C" "RA_Infinite" (Class|FGResourceNode|GetResoucePurity))
      (CallFunction|CreateInstances))))

(fn ConstructionScript)

(fn CreateInstances
  (bind _returnvalue (Math|Random|RandomFloatinRange 1.0 2.0))
  (for _index (range 0 8)
    (Components|InstancedStaticMesh|AddInstance (Variables|Default|GetPillsMesh) (Math|Transform|MakeTransform (Math|Vector|RotateVectorAroundAxis (Math|Vector|MakeVector (* 8e+02 (Math|Curves|GetFloatValue (Variables|Components|GetPileShape) (Math|Random|RandomFloat))) 0.0 0.0) (Math|Random|RandomFloatinRange 0.0 3.6e+02) "0.000000,0.000000,1.000000") "0, 0, 0" (Math|Vector|MakeVector _returnvalue _returnvalue _returnvalue)) false)))